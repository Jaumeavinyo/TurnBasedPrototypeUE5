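; Player Blueprint that starts with a greatsword on its back and supports drawing and sheathing it.
; On BeginPlay it equips BP_GreatSwordWeapon to the back socket through the Weapon component if no valid weapon is set.
; Two debug keys call DrawWeapon and SheatheWeapon.
; Custom events intended for anim notifies move the weapon between the right-hand and back sockets.
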(event Custom|CustomEvent_DrawWeapon
  ;[1 0.7719 0.7719 0.5] CUSTOM EVENTS: ANIM NOTIFY
  (Class|WeaponComponent|SetCurrentSocket (Variables|Default|GetWeapon) "SwordOnRHand"))

(event Custom|CustomEvent_SheatheWeapon
  ;[1 0.7719 0.7719 0.5] CUSTOM EVENTS: ANIM NOTIFY
  (Class|WeaponComponent|SetCurrentSocket (Variables|Default|GetWeapon) "SwordOnBack"))

(event EventBeginPlay
  (bind _weapon (Variables|Default|GetWeapon))
  (Utilities|IsValid (Class|WeaponComponent|GetCurrentWeapon _weapon)
    (:Is%20Not%20Valid
      (Class|WeaponComponent|EquipWeapon _weapon "/Game/BG3_Game/Weapons/GreatSword/BP_GreatSwordWeapon.BP_GreatSwordWeapon_C" "SwordOnBack"))))

(event Collision|EventActorBeginOverlap
  (params (OtherActor :type Actor%20Object%20Reference)))

(event EventTick
  (params (DeltaSeconds :type Float%20%28single-precision%29)))

(event Input|KeyboardEvents|DebugKey1
  (params (Key :type Key%20Structure :default "None") (ActionValue :type Input%20Action%20Value%20Structure))
  (:Pressed
    (Class|BaseCharacter|DrawWeapon "None")))

(event Input|KeyboardEvents|DebugKey2
  (params (Key :type Key%20Structure :default "None") (ActionValue :type Input%20Action%20Value%20Structure))
  (:Pressed
    (Class|BaseCharacter|SheatheWeapon "None")))

(fn ConstructionScript)