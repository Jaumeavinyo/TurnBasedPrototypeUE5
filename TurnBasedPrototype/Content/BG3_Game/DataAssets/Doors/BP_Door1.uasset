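; BP_Door1 is a door actor that swings its mesh open or closed through a StartRotation event.
; The DoorMovement timeline plays from the start and offsets the mesh's relative yaw from InitialYaw, in the negative direction to open and positive to close.
; InitialYaw is cached at BeginPlay and again when the timeline finishes, so each swing is relative to where the last one ended.
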(event `self.StartRotation`
  (params (bToOpen :type Boolean))
  (bind (_direction _rotationvalue) (`Timeline|DoorMovement` :!via `PlayFromStart`)
    (:`Update`
      (if bToOpen
        (`SceneComponent.K2_SetRelativeRotation` (`self.DoorMeshComponent`) (`KismetMathLibrary.MakeRotator` 0.0 0.0 (+ (`self.initialYaw`) (* _rotationvalue -1.0))) false false)
        (else
          (`SceneComponent.K2_SetRelativeRotation` (`self.DoorMeshComponent`) (`KismetMathLibrary.MakeRotator` 0.0 0.0 (+ (`self.initialYaw`) _rotationvalue)) false false))))
    (:`Finished`
      (set `self.initialYaw` (.yaw (.rotation (`SceneComponent.GetRelativeTransform` (`self.DoorMeshComponent`))))))))

(event `self.ReceiveTick`
  (params (DeltaSeconds :type "Float (single-precision)")))

(event `self.ReceiveBeginPlay`
  (set `self.initialYaw` (.yaw (.rotation (`SceneComponent.GetRelativeTransform` (`self.DoorMeshComponent`))))))

(fn `UserConstructionScript`)